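; Mirror actor that makes an entity appear when the player enters its collision and launches a minigame.
; If the game mode's CanSpawnEntity flag is set, it clears the flag and a random looping MultiGate reveals the businessman or scared bully decal.
; After a short delay, the game mode starts minigame A or B to match the decal.
; A DespawnEntity event hides both decals.
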(event OnComponentBeginOverlap(Mirror_Collision)
  (params (OverlappedComponent :type Primitive%20Component%20Object%20Reference) (OtherActor :type Actor%20Object%20Reference) (OtherComp :type Primitive%20Component%20Object%20Reference) (OtherBodyIndex :type Integer) (bFromSweep :type Boolean) (SweepResult :type Hit%20Result%20Structure%20%28by%20ref%29))
  ;[0.15 0.15 0.15 0.5] Logica para que aparezcan entidades
  (Utilities|Casting|CastToBP_PlayerCharacter OtherActor)
  (bind _asbp_first_person_game_mode (Utilities|Casting|CastToBP_FirstPersonGameMode (Game|GetGameMode)))
  (if (Variables|/Game/FirstPerson/Blueprints/BP_FirstPersonGameMode.BP_FirstPersonGameMode_C|GetCanSpawnEntity? _asbp_first_person_game_mode)
    (Variables|/Game/FirstPerson/Blueprints/BP_FirstPersonGameMode.BP_FirstPersonGameMode_C|SetCanSpawnEntity? _asbp_first_person_game_mode false)
    (Development|PrintString "Se spawnea entidad")
    (Utilities|FlowControl|MultiGate true true -1
      (:Out%200
        (Rendering|SetVisibility (Variables|Default|GetDecal_BusinessMan) true false)
        (Utilities|FlowControl|Delay 2.0)
        (bind _asbp_first_person_game_mode_2 (Utilities|Casting|CastToBP_FirstPersonGameMode (Game|GetGameMode)))
        (Default|StartMinigameA _asbp_first_person_game_mode_2))
      (:Out%201
        (Rendering|SetVisibility (Variables|Default|GetDecal_BullyScared) true false)
        (Utilities|FlowControl|Delay 2.0)
        (bind _asbp_first_person_game_mode_3 (Utilities|Casting|CastToBP_FirstPersonGameMode (Game|GetGameMode)))
        (Default|StartMinigameB _asbp_first_person_game_mode_3)))
    (else
      (Development|PrintString "No se spawnea entidad")
      (Utilities|FlowControl|Delay 2.0)
      (Variables|/Game/FirstPerson/Blueprints/BP_FirstPersonGameMode.BP_FirstPersonGameMode_C|SetCanSpawnEntity? _asbp_first_person_game_mode false))))

(event Custom|DespawnEntity
  ;[0.15 0.15 0.15 0.5] Logica para hacer desaparecer entidades
  (Rendering|SetVisibility (Variables|Default|GetDecal_BusinessMan) false false)
  (Rendering|SetVisibility (Variables|Default|GetDecal_BullyScared) false false)
  (Utilities|FlowControl|Delay 2.0))

(event EventBeginPlay
  ;[0.15 0.15 0.15 0.5] Setear Referencia al Player al iniciar juego
  (bind _asbp_player_character (Utilities|Casting|CastToBP_PlayerCharacter (Game|GetPlayerCharacter 0)))
  (Variables|Default|SetBPPlayerCharRef _asbp_player_character))

(fn ConstructionScript)